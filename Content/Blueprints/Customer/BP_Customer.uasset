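; BP_Customer is a customer whose final emotion is decided by a four-step, keyboard-driven dialogue.
; While enabled, keys 1 and 3 raise or lower EmotionProgress, count the response and set CanUseLights.
; The fourth response disables further choices and prints FirstEmotion or SecondEmotion as FinalEmotion, but only if the score's sign matches that last key.
; BeginPlay enables player-zero input directly on the actor.
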(event EventBeginPlay
  (Input|EnableInput (Game|GetPlayerController 0)))

(event EventTick
  (params (DeltaSeconds :type Float%20%28single-precision%29)))

(event Input|KeyboardEvents|1
  (params (Key :type Key%20Structure :default "None"))
  (bind _dialoguecounter (Variables|Default|GetDialogueCounter))
  (:Pressed
    (if (Variables|Default|GetisEnabled)
      (if (< (Variables|Default|GetDialogueCounter) 4)
        (bind _result (Math|Integer|IncrementInt (Variables|Default|GetEmotionProgress))
          (:%20%20
            (Development|PrintString (Utilities|String|ToString(Integer) _result))
            (Math|Integer|IncrementInt _dialoguecounter
              (:%20%20
                (Variables|Default|SetCanUseLights true)
                (if (== _dialoguecounter 4)
                  (Variables|Default|SetisEnabled false)
                  (Variables|Default|SetCanUseLights true)
                  (if (> (Variables|Default|GetEmotionProgress) 0)
                    (bind _output_get (Variables|Default|SetFinalEmotion (Variables|Default|GetFirstEmotion)))
                    (Development|PrintString (Utilities|String|EnumtoString _output_get))))))))))))

(event Input|KeyboardEvents|3
  (params (Key :type Key%20Structure :default "None"))
  (bind _dialoguecounter (Variables|Default|GetDialogueCounter))
  (:Pressed
    (if (Variables|Default|GetisEnabled)
      (if (< (Variables|Default|GetDialogueCounter) 4)
        (bind _result (Math|Integer|DecrementInt (Variables|Default|GetEmotionProgress))
          (:%20%20
            (Development|PrintString (Utilities|String|ToString(Integer) _result))
            (Math|Integer|IncrementInt _dialoguecounter
              (:%20%20
                (Variables|Default|SetCanUseLights true)
                (if (== _dialoguecounter 4)
                  (Variables|Default|SetisEnabled false)
                  (Variables|Default|SetCanUseLights true)
                  (if (< (Variables|Default|GetEmotionProgress) 0)
                    (bind _output_get (Variables|Default|SetFinalEmotion (Variables|Default|GetSecondEmotion)))
                    (Development|PrintString (Utilities|String|EnumtoString _output_get))))))))))))

(fn ConstructionScript)